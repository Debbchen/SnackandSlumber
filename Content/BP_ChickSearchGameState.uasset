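; BP_ChickSearchGameState is the game state for a chick-collecting game, tracking progress and the win condition.
; On BeginPlay it counts all BP_Chick actors in the level to set the total.
; Each AddChick call increments the collected count and compares it to that total.
; On a match it flags the game as won, switches input to UI-only, shows the cursor and stops the BP_Fox player pawn's movement.
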(event Custom|AddChick
  (bind _returnvalue (Game|GetPlayerController 0))
  ;[0.15 0.15 0.15 0.5] Kücken aufsammeln
  (Variables|Default|SetCollectedChickNumber (+ (Variables|Default|GetCollectedChickNumber) 1))
  ;[0.15 0.15 0.15 0.5] Prüfen ob alle Kücken aufgesammelt sind
  (if (== (Variables|Default|GetCollectedChickNumber) (Variables|Default|GetTotalChickNumber))
    (Variables|Default|SetGameWon true)
    (Input|SetInputModeUIOnly _returnvalue 0 "DoNotLock" false)
    (Variables|/Script/Engine.PlayerController|SetbShowMouseCursor _returnvalue true)
    (bind _asbp_fox (Utilities|Casting|CastToBP_Fox (Game|Player|GetPlayerPawn 0)))
    (Default|StopFoxMovement _asbp_fox)))

(event EventBeginPlay
  ;[0.15 0.15 0.15 0.5] Kücken im Level zählen
  (bind _outactors (Actor|GetAllActorsOfClass "/Game/Characters/Chick/BP_Chick.BP_Chick_C"))
  (Variables|Default|SetTotalChickNumber (Utilities|Array|Length _outactors)))

(fn ConstructionScript)