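; BP_Chick is a collectible chick that flees from the player (the fox) until caught.
; A looping timer checks horizontal distance, launching the chick away with random strength and a jump cooldown, plus an AIMoveTo toward the navmesh-projected flee point.
; Out of range, it stops controller movement.
; Player overlap plays pickup sound and effects, increments the count in BP_ChickSearchGameState via AddChick, and destroys the chick.
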(event Custom|Fluchtpruefen
  (bind _returnvalue (Game|Player|GetPlayerPawn 0))
  (bind _returnvalue_2 (Pawn|GetController))
  (bind _self self)
  (bind _returnvalue_3 (Transformation|GetActorLocation _self))
  ;[0.15 0.15 0.15 0.5] Flucht vor dem Fuchs
  ;;[0.15 0.15 0.15 0.5] Fuchs erkennen und Flucht auslösen
  (Utilities|IsValid _returnvalue
    (:Is%20Valid
      (if (< (Transformation|GetHorizontalDistanceTo _returnvalue) 5e+02)
        ;;[0.15 0.15 0.15 0.5] Fluchtsprung ausführen
        (if (and (Character|CanJump) (Variables|Default|GetSprungbereit))
          (Variables|Default|SetSprungbereit false)
          (Variables|Default|SetAktuelleSprungweite (Math|Random|RandomFloatinRange 4.5e+03 7.5e+03))
          (Transformation|SetActorRotation (Math|Rotator|MakeRotfromX (* (Math|Vector|GetUnitDirection(Vector) (Transformation|GetActorLocation _returnvalue) _returnvalue_3) (Math|Vector|MakeVector (Variables|Default|GetAktuelleSprungweite) (Variables|Default|GetAktuelleSprungweite) 0.0))))
          (Audio|SpawnSoundatLocation "/Game/Audio/SoundEffects/S_Grasshopper_Jump.S_Grasshopper_Jump" (Transformation|GetActorLocation) "0, 0, 0" 0.1 1.0 0.0 0 0)
          (Character|LaunchCharacter (+ (* (Math|Vector|GetUnitDirection(Vector) (Transformation|GetActorLocation _returnvalue) _returnvalue_3) (Math|Vector|MakeVector (Variables|Default|GetAktuelleSprungweite) (Variables|Default|GetAktuelleSprungweite) 0.0)) "0.000000,0.000000,500.000000") true true)
          ;;;[0.15 0.15 0.15 0.5] Sprung-Cooldown
          (Utilities|FlowControl|Sequence
            (:then_0
              (if (.ReturnValue (AI|Navigation|ProjectPointtoNavigation (+ (* (Math|Vector|GetUnitDirection(Vector) (Transformation|GetActorLocation _returnvalue) _returnvalue_3) (Math|Vector|MakeVector (Variables|Default|GetAktuelleSprungweite) (Variables|Default|GetAktuelleSprungweite) 0.0)) _returnvalue_3) 0 0 "200.000000,200.000000,500.000000"))
                ;;[0.15 0.15 0.15 0.5] Fluchtziel berechnen
                (AI|AIMoveTo _self (.ProjectedLocation (AI|Navigation|ProjectPointtoNavigation (+ (* (Math|Vector|GetUnitDirection(Vector) (Transformation|GetActorLocation _returnvalue) _returnvalue_3) (Math|Vector|MakeVector (Variables|Default|GetAktuelleSprungweite) (Variables|Default|GetAktuelleSprungweite) 0.0)) _returnvalue_3) 0 0 "200.000000,200.000000,500.000000")) 0 3e+01 false)))
            (:then_1
              (Utilities|FlowControl|Delay 1.5)
              (Variables|Default|SetSprungbereit true))))
        (else
          ;;[0.15 0.15 0.15 0.5] Außerhalb der Fluchtdistanz anhalten
          (Utilities|IsValid _returnvalue_2
            (:Is%20Valid
              (AI|Navigation|StopMovement _returnvalue_2))))))))

(event EventBeginPlay
  ;[0.15 0.15 0.15 0.5] Flucht vor dem Fuchs
  ;;[0.15 0.15 0.15 0.5] Fuchs erkennen und Flucht auslösen
  (Utilities|Time|SetTimerbyEvent (delegate Custom|Fluchtpruefen) 0.3 true))

(event Collision|EventActorBeginOverlap
  (params (OtherActor :type Actor%20Object%20Reference))
  ;[0.15 0.15 0.15 0.5] Grashüpfer einsammeln
  (if (== OtherActor (Game|Player|GetPlayerPawn 0))
    (Development|PrintString "Kücken aufgesammelt")
    (Audio|SpawnSoundatLocation "/Game/Audio/SoundEffects/SC_Ha.SC_Ha" (Transformation|GetActorLocation) "0, 0, 0" 1.0 1.0 0.0 0 0)
    (Niagara|SpawnSystematLocation "/Game/Characters/Chick/PS_PickUp.PS_PickUp" (Transformation|GetActorLocation))
    ;;[0.15 0.15 0.15 0.5] Grashüpfer Zähler hochzählen
    (bind _asbp_chick_search_game_state (Utilities|Casting|CastToBP_ChickSearchGameState (Game|GetGameState)))
    (Default|AddChick _asbp_chick_search_game_state)
    (Actor|DestroyActor)))

(event EventTick
  (params (DeltaSeconds :type Float%20%28single-precision%29)))

(fn ConstructionScript)